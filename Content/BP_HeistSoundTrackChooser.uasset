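; Main-menu actor for a heist soundtrack jukebox mod, destroying itself outside the menu game mode or when the heist chooser actor exists.
; BeginPlay loads songs into a shared persistent object and plays the custom menu theme, guarded against restarts.
; Lobby state-machine events swap pre-heist and jukebox widgets.
; Settings and playlist persist in a save slot, recreated if invalid, with playlist soft references validated on load.
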(event `self.ReceiveDestroyed`
  (`Widget.RemoveFromParent` (`self.PreHeistWidget`)))

(event `self.ReceiveBeginPlay`
  (bind _returnvalue (`SBZMusicManager.GetMusicManager`))
  (bind _returnvalue_2 (`SBZGameStateMachineFunctionLibrary.GetGameStateMachine`))
  (bind _as_heist_soundtrack_persistent_object (`self.As Heist Soundtrack Persistent Object`))
  (`/PDML/Blueprints/Utilities/BPFL_ModLoader.PrintToModLoader` "Jukebox menu actor BeginPlay")
  (bind _returnvalue_3 (`GameplayStatics.GetActorOfClass` "/JukeboxMod/BP_OnHeistSoundTrackChooser.BP_OnHeistSoundTrackChooser_C"))
  (if (or (`KismetSystemLibrary.IsValid` _returnvalue_3) (not (`.bSuccess` (cast `SBZGameModeMainMenu` (`GameplayStatics.GetGameMode`) :!pure true))))
    (`/PDML/Blueprints/Utilities/BPFL_ModLoader.PrintToModLoader` "Heist actor found destroying menu actor")
    (`self.K2_DestroyActor`)
    (else
      (bind _persistentobject (`/JukeboxMod/BPML_Jukebox.GetPersistentObject`)
        (:`Found`
          (set `self.As Heist Soundtrack Persistent Object` _persistentobject)
          (bind (_initalsong _initialmenusong) (`/JukeboxMod/JukeboxFuncLibrary.LoadSongs`))
          (set `/JukeboxMod/HeistSoundtrackPersistentObject.PDAHeist` _initalsong _as_heist_soundtrack_persistent_object)
          (bind _output_get (set `/JukeboxMod/HeistSoundtrackPersistentObject.PDAMenu` _initialmenusong _as_heist_soundtrack_persistent_object))
          (if (not (or (`/JukeboxMod/HeistSoundtrackPersistentObject.IsPlayingCustomMenuTheme` _as_heist_soundtrack_persistent_object) (== (`/JukeboxMod/HeistSoundtrackPersistentObject.PDAMenu` _as_heist_soundtrack_persistent_object) "/JukeboxMod/Music/Menu/MenuTheme.MenuTheme")))
            (`SBZMusicManager.StopMusic` _returnvalue)
            (`SBZMusicManager.PlayMusic` _returnvalue (`/JukeboxMod/PDA_MenuSoundtrack.Audio Event` _output_get) false)
            (set `/JukeboxMod/HeistSoundtrackPersistentObject.IsPlayingCustomMenuTheme` true (`self.As Heist Soundtrack Persistent Object`)))
          (`self.SetupSave`)
          (add `SBZGameStateMachine.OnStateMachineEnteredLobby` _returnvalue_2 (`|CreateDelegate` :!event `JoinedLobbyEvent`))
          (add `SBZGameStateMachine.OnStateMachineExitedLobby` _returnvalue_2 (`|CreateDelegate` :!event `ExitedLobbyEvent`))
          (`self.ExitedLobbyEvent`)
          (add `/JukeboxMod/HeistSoundtrackPersistentObject.CallSaveGame` (`self.As Heist Soundtrack Persistent Object`) (`|CreateDelegate` :!event `CallSaveGame`))
          (`/PDML/Blueprints/Utilities/BPFL_ModLoader.PrintToModLoader` "Jukebox menu actor BeginPlay Finished"))
        (:`NotFound`
          (`/PDML/Blueprints/Utilities/BPFL_ModLoader.PrintToModLoader` "FAILED TO FIND HEIST SOUNDTRACK OBJECT"))))))

(event `ExitedLobbyEvent`
  (`/PDML/Blueprints/Utilities/BPFL_ModLoader.PrintToModLoader` "ExitedLobbyEvent")
  (bind _preheistwidget (`self.PreHeistWidget`)
    (:`then`
      (`Widget.RemoveFromParent` _preheistwidget))
    (:`else`
      _))
  (bind _returnvalue (`|CreateWidget` "/JukeboxMod/Widgets/JukeboxPreHeistWidget.JukeboxPreHeistWidget_C"))
  (`UserWidget.AddToViewport` _returnvalue 9999)
  (set `self.PreHeistWidget` _returnvalue))

(event `JoinedLobbyEvent`
  (`/PDML/Blueprints/Utilities/BPFL_ModLoader.PrintToModLoader` "JoinLobbyEvent")
  (`Widget.RemoveFromParent` (`self.PreHeistWidget`))
  (set `/JukeboxMod/HeistSoundtrackPersistentObject.JukeboxDisabled` false (`self.As Heist Soundtrack Persistent Object`))
  (`/JukeboxMod/JukeboxFuncLibrary.SetDefaultForHeist` (`SBZGameStateMachineFunctionLibrary.GetGameStateMachine`))
  (bind _returnvalue (`|CreateWidget` "/JukeboxMod/Widgets/JukeboxWidget.JukeboxWidget_C"))
  (`UserWidget.AddToViewport` _returnvalue 9999))

(event `CallSaveGame`
  (`/PDML/Blueprints/Utilities/BPFL_ModLoader.PrintToModLoader` "CallSaveGame")
  (`self.Save`))

(fn `LoadSave`
  (bind _as_heist_soundtrack_persistent_object (`self.As Heist Soundtrack Persistent Object`))
  (bind _pdaheistplaylistarray (`/JukeboxMod/HeistJukeboxSaveGame.PDAHeistPlaylistArray` (`self.SaveGameObject`)))
  (`/PDML/Blueprints/Utilities/BPFL_ModLoader.PrintToModLoader` "Loading")
  (bind _savegameobject (`self.SaveGameObject`)
    (:`then`
      ;[1 1 1] loads all those variables that are supposed to be saved
      (bind _as_heist_soundtrack_persistent_object_2 (`self.As Heist Soundtrack Persistent Object`)
        (:`then`
          (set `self.SaveLoaded` (`/JukeboxMod/HeistJukeboxSaveGame.Exists` _savegameobject))
          (bind _output_get (set `/JukeboxMod/HeistSoundtrackPersistentObject.randomSong` (`/JukeboxMod/HeistJukeboxSaveGame.RandomEnabled` _savegameobject) _as_heist_soundtrack_persistent_object_2))
          (bind _output_get_2 (set `/JukeboxMod/HeistSoundtrackPersistentObject.assaultRandomSong` (`/JukeboxMod/HeistJukeboxSaveGame.RandomAssaultEnabled` _savegameobject) _as_heist_soundtrack_persistent_object_2))
          (bind _output_get_3 (set `/JukeboxMod/HeistSoundtrackPersistentObject.playlistEnabled` (`/JukeboxMod/HeistJukeboxSaveGame.PlaylistEnabled` _savegameobject) _as_heist_soundtrack_persistent_object_2))
          (bind _output_get_4 (set `/JukeboxMod/HeistSoundtrackPersistentObject.disableRTCFix` (`/JukeboxMod/HeistJukeboxSaveGame.RTCFixDisabled` _savegameobject) _as_heist_soundtrack_persistent_object_2))
          (bind _output_get_5 (set `/JukeboxMod/HeistSoundtrackPersistentObject.EnableRTCStealth` (`/JukeboxMod/HeistJukeboxSaveGame.RTCStealthEnabled` _savegameobject) _as_heist_soundtrack_persistent_object_2))
          (bind _output_get_6 (set `/JukeboxMod/HeistSoundtrackPersistentObject.EnableEndlessRanTrack` (`/JukeboxMod/HeistJukeboxSaveGame.EnableEndlessRanTrack` _savegameobject) _as_heist_soundtrack_persistent_object_2))
          (bind _output_get_7 (set `/JukeboxMod/HeistSoundtrackPersistentObject.UseAltTrackNames` (`/JukeboxMod/HeistJukeboxSaveGame.UseAltTrackNames` _savegameobject) _as_heist_soundtrack_persistent_object_2))
          (`/PDML/Blueprints/Utilities/BPFL_ModLoader.PrintToModLoader` (`KismetStringLibrary.Concat_StrStr` (`KismetStringLibrary.Conv_BoolToString` _output_get) (`KismetStringLibrary.Conv_BoolToString` _output_get_2) (`KismetStringLibrary.Conv_BoolToString` _output_get_3) (`KismetStringLibrary.Conv_BoolToString` _output_get_4) (`KismetStringLibrary.Conv_BoolToString` _output_get_5) (`KismetStringLibrary.Conv_BoolToString` _output_get_6) (`KismetStringLibrary.Conv_BoolToString` _output_get_7)))
          (if (`/JukeboxMod/HeistSoundtrackPersistentObject.playlistEnabled` _as_heist_soundtrack_persistent_object_2)
            (for _array_element _pdaheistplaylistarray
              (if (`KismetSystemLibrary.IsValidSoftObjectReference` _array_element)
                (bind _returnvalue (`KismetSystemLibrary.LoadAsset_Blocking` _array_element))
                (`/Engine/EditorBlueprintResources/StandardMacros.IsValid` _returnvalue
                  (:`Is Valid`
                    (for _array_element_2 (`/JukeboxMod/HeistSoundtrackPersistentObject.PDAHeistSoundtrackarray` _as_heist_soundtrack_persistent_object)
                      (if (== _array_element_2 _returnvalue)
                        (`KismetArrayLibrary.Array_AddUnique` (`/JukeboxMod/HeistSoundtrackPersistentObject.PDAHeistPlaylistArray` _as_heist_soundtrack_persistent_object) _array_element_2)
                        (`/PDML/Blueprints/Utilities/BPFL_ModLoader.PrintToModLoader` (`KismetSystemLibrary.GetDisplayName` _array_element_2)))))
                  (:`Is Not Valid`
                    (`/PDML/Blueprints/Utilities/BPFL_ModLoader.PrintToModLoader` "Invalid object")
                    (`KismetArrayLibrary.Array_RemoveItem` _pdaheistplaylistarray _array_element)))
                (else
                  (`/PDML/Blueprints/Utilities/BPFL_ModLoader.PrintToModLoader` "Invalid soft reference")
                  (`KismetArrayLibrary.Array_RemoveItem` _pdaheistplaylistarray _array_element)))))
          (`/PDML/Blueprints/Utilities/BPFL_ModLoader.PrintToModLoader` "Loaded"))
        (:`else`
          (`/PDML/Blueprints/Utilities/BPFL_ModLoader.PrintToModLoader` "Persistent object invalid"))))
    (:`else`
      (`/PDML/Blueprints/Utilities/BPFL_ModLoader.PrintToModLoader` "SaveGameObject invalid"))))

(fn `Save`
  (bind _as_heist_soundtrack_persistent_object (`self.As Heist Soundtrack Persistent Object`))
  (bind _pdaheistplaylistarray (`/JukeboxMod/HeistSoundtrackPersistentObject.PDAHeistPlaylistArray` (`self.As Heist Soundtrack Persistent Object`)))
  (`/PDML/Blueprints/Utilities/BPFL_ModLoader.PrintToModLoader` "Saving")
  ;[1 1 1] there has to be a better way to do this
  (bind _savegameobject (`self.SaveGameObject`)
    (:`then`
      (bind _as_heist_soundtrack_persistent_object_2 (`self.As Heist Soundtrack Persistent Object`)
        (:`then`
          (bind _output_get (set `/JukeboxMod/HeistJukeboxSaveGame.RandomEnabled` (`/JukeboxMod/HeistSoundtrackPersistentObject.randomSong` _as_heist_soundtrack_persistent_object_2) _savegameobject))
          (bind _output_get_2 (set `/JukeboxMod/HeistJukeboxSaveGame.RandomAssaultEnabled` (`/JukeboxMod/HeistSoundtrackPersistentObject.assaultRandomSong` _as_heist_soundtrack_persistent_object_2) _savegameobject))
          (bind _output_get_3 (set `/JukeboxMod/HeistJukeboxSaveGame.PlaylistEnabled` (`/JukeboxMod/HeistSoundtrackPersistentObject.playlistEnabled` _as_heist_soundtrack_persistent_object_2) _savegameobject))
          (bind _output_get_4 (set `/JukeboxMod/HeistJukeboxSaveGame.RTCStealthEnabled` (`/JukeboxMod/HeistSoundtrackPersistentObject.EnableRTCStealth` _as_heist_soundtrack_persistent_object_2) _savegameobject))
          (bind _output_get_5 (set `/JukeboxMod/HeistJukeboxSaveGame.RTCFixDisabled` (`/JukeboxMod/HeistSoundtrackPersistentObject.disableRTCFix` _as_heist_soundtrack_persistent_object_2) _savegameobject))
          (bind _output_get_6 (set `/JukeboxMod/HeistJukeboxSaveGame.EnableEndlessRanTrack` (`/JukeboxMod/HeistSoundtrackPersistentObject.EnableEndlessRanTrack` _as_heist_soundtrack_persistent_object_2) _savegameobject))
          (bind _output_get_7 (set `/JukeboxMod/HeistJukeboxSaveGame.UseAltTrackNames` (`/JukeboxMod/HeistSoundtrackPersistentObject.UseAltTrackNames` _as_heist_soundtrack_persistent_object_2) _savegameobject))
          (if (`/JukeboxMod/HeistJukeboxSaveGame.PlaylistEnabled` (`self.SaveGameObject`))
            (if (>= (`KismetArrayLibrary.Array_Length` _pdaheistplaylistarray) 1)
              (for _array_element _pdaheistplaylistarray
                (`KismetArrayLibrary.Array_AddUnique` (`/JukeboxMod/HeistJukeboxSaveGame.PDAHeistPlaylistArray` (`self.SaveGameObject`)) (`|ConvertAsset` _array_element)))
              (else
                (set `/JukeboxMod/HeistJukeboxSaveGame.PlaylistEnabled` false (`self.SaveGameObject`))
                (set `/JukeboxMod/HeistSoundtrackPersistentObject.playlistEnabled` false _as_heist_soundtrack_persistent_object)
                (`/JukeboxMod/HeistSoundtrackPersistentObject.PlaylistTrackToggled` _as_heist_soundtrack_persistent_object false)
                (`KismetArrayLibrary.Array_Clear` (`/JukeboxMod/HeistJukeboxSaveGame.PDAHeistPlaylistArray` (`self.SaveGameObject`)) :!label _label)))
            (else
              (goto _label)))
          (`/PDML/Blueprints/Utilities/BPFL_ModLoader.PrintToModLoader` (`KismetStringLibrary.Concat_StrStr` (`KismetStringLibrary.Conv_BoolToString` _output_get) (`KismetStringLibrary.Conv_BoolToString` _output_get_2) (`KismetStringLibrary.Conv_BoolToString` _output_get_3) (`KismetStringLibrary.Conv_BoolToString` _output_get_4) (`KismetStringLibrary.Conv_BoolToString` _output_get_5) (`KismetStringLibrary.Conv_BoolToString` _output_get_6) (`KismetStringLibrary.Conv_BoolToString` _output_get_7)))
          (bind _returnvalue (`GameplayStatics.SaveGameToSlot` (`self.SaveGameObject`) "HeistJukeboxSaveGame"))
          (if _returnvalue
            (`/PDML/Blueprints/Utilities/BPFL_ModLoader.PrintToModLoader` "Saved")
            (else
              (`/PDML/Blueprints/Utilities/BPFL_ModLoader.PrintToModLoader` "Failed to save")))
          (return))
        (:`else`
          (`/PDML/Blueprints/Utilities/BPFL_ModLoader.PrintToModLoader` "Persistent object invalid"))))
    (:`else`
      (`/PDML/Blueprints/Utilities/BPFL_ModLoader.PrintToModLoader` "SaveGameObject invalid"))))

(fn `SetupSave`
  (bind _returnvalue (`GameplayStatics.DoesSaveGameExist` "HeistJukeboxSaveGame"))
  (if _returnvalue
    (bind _returnvalue_2 (`GameplayStatics.LoadGameFromSlot` "HeistJukeboxSaveGame"))
    (bind _asheist_jukebox_save_game (cast `/JukeboxMod/HeistJukeboxSaveGame` _returnvalue_2)
      (:`then`
        (set `self.SaveGameObject` _asheist_jukebox_save_game)
        (`self.LoadSave`)
        (if (`self.SaveLoaded`)
          (`/PDML/Blueprints/Utilities/BPFL_ModLoader.PrintToModLoader` "Save loaded")
          (else
            (`GameplayStatics.DeleteGameInSlot` "HeistJukeboxSaveGame" :!label _label)
            (set `self.SaveLoaded` true)
            (`/PDML/Blueprints/Utilities/BPFL_ModLoader.PrintToModLoader` "Save doesnt exist loading" :!label _label_2)
            (bind _returnvalue_3 (`GameplayStatics.CreateSaveGameObject` "/JukeboxMod/HeistJukeboxSaveGame.HeistJukeboxSaveGame_C"))
            (bind _output_get (set `self.SaveGameObject` _returnvalue_3))
            (set `/JukeboxMod/HeistJukeboxSaveGame.Exists` true _output_get)
            (`GameplayStatics.SaveGameToSlot` _output_get "HeistJukeboxSaveGame")
            (`/PDML/Blueprints/Utilities/BPFL_ModLoader.PrintToModLoader` "Save loaded"))))
      (:`CastFailed`
        (`/PDML/Blueprints/Utilities/BPFL_ModLoader.PrintToModLoader` "Savegame cast failed")
        (goto _label)))
    (else
      (goto _label_2))))

(fn `UserConstructionScript`)