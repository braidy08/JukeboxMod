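; In-heist jukebox actor for a PD3 mod that plays custom heist soundtracks using settings from a persistent object.
; On BeginPlay it loads songs and widgets, skips tutorials, then polls for ActionPhase before playing the track.
; Heist state changes can reroll tracks (retry-capped to avoid stealth-only songs) and start double-time, optionally endless random music at Point of No Return.
; RTCFix silences diegetic nightclub music on the RTC heist.
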(event `self.ReceiveBeginPlay`
  (bind _as_heist_soundtrack_persistent_object (`self.As Heist Soundtrack Persistent Object`))
  (bind _as_heist_soundtrack_persistent_object_2 (`self.As Heist Soundtrack Persistent Object`))
  (`/PDML/Blueprints/Utilities/BPFL_ModLoader.PrintToModLoader` "Jukebox game actor BeginPlay")
  (bind _persistentobject (`/JukeboxMod/BPML_Jukebox.GetPersistentObject`)
    (:`Found`
      (set `self.As Heist Soundtrack Persistent Object` _persistentobject)
      (if (`/JukeboxMod/HeistSoundtrackPersistentObject.JukeboxDisabled` _as_heist_soundtrack_persistent_object_2)
        (`/PDML/Blueprints/Utilities/BPFL_ModLoader.PrintToModLoader` "Jukebox Disabled")
        (else
          (set `/JukeboxMod/HeistSoundtrackPersistentObject.IsPlayingCustomMenuTheme` false _as_heist_soundtrack_persistent_object_2)
          (`/JukeboxMod/JukeboxFuncLibrary.LoadSongs`)
          (bind _returnvalue (`GameplayStatics.GetActorOfClass` "/Script/Starbreeze.PD3HeistGameState"))
          (set `self.PD3HeistGameState` _returnvalue)
          (`/PDML/Blueprints/Utilities/BPFL_ModLoader.PrintToModLoader` "Loaded Jukebox")
          (`self.SetupInHeistWidgets`)
          (`self.SetupDebugStuff`)
          (bind _validheist (`self.GetCurrentHeist`))
          (if _validheist
            (if (`/JukeboxMod/HeistSoundtrackPersistentObject.randomSong` (`self.As Heist Soundtrack Persistent Object`))
              (`/JukeboxMod/JukeboxFuncLibrary.SelectRandomTrack`))
            (if (`|EnumEquality` (`SBZGameStateMachineFunctionLibrary.GetGameStateMachineState`) "SM_ActionPhase") :!label _label
              (`self.RTC_Fix`)
              (`KismetSystemLibrary.Delay` 1.0)
              (`/JukeboxMod/JukeboxFuncLibrary.PlaySong` (`/JukeboxMod/HeistSoundtrackPersistentObject.PDAHeist` _as_heist_soundtrack_persistent_object))
              (if (or (`/JukeboxMod/HeistSoundtrackPersistentObject.assaultRandomSong` _as_heist_soundtrack_persistent_object) (`/JukeboxMod/HeistSoundtrackPersistentObject.playlistEnabled` _as_heist_soundtrack_persistent_object) (`/JukeboxMod/HeistSoundtrackPersistentObject.HeistIsRTC` _as_heist_soundtrack_persistent_object))
                (add `PD3HeistGameState.OnHeistStateChanged` (`self.PD3HeistGameState`) (`|CreateDelegate` :!event `OnHeistStateChanged`)))
              (else
                (`KismetSystemLibrary.Delay` 0.2)
                (goto _label)))
            (else
              (`/PDML/Blueprints/Utilities/BPFL_ModLoader.PrintToModLoader` "invalid heist"))))))
    (:`NotFound`
      (`/PDML/Blueprints/Utilities/BPFL_ModLoader.PrintToModLoader` "FAILED TO FIND HEIST SOUNDTRACK OBJECT"))))

(event `OnHeistStateChanged`
  (params (OldState :type "EPD3HeistState Enum" :default "Stealth") (NewState :type "EPD3HeistState Enum" :default "Stealth"))
  (bind _stealthreselectattempts (`self.StealthReselectAttempts`))
  (bind _pdaheist (`/JukeboxMod/HeistSoundtrackPersistentObject.PDAHeist` (`self.As Heist Soundtrack Persistent Object`)))
  (`self.HeistStateChangedEvent` OldState NewState)
  (if (`|EnumEquality` NewState "PointOfNoReturn")
    (`SBZMusicManager.SetSwitch` (`SBZMusicManager.GetMusicManager`) "music_switch_special" "doubletime")
    (if (`/JukeboxMod/HeistSoundtrackPersistentObject.EnableEndlessRanTrack` (`self.As Heist Soundtrack Persistent Object`))
      (`/JukeboxMod/JukeboxFuncLibrary.SelectRandomTrack` :!label _label_2)
      (if (<= _stealthreselectattempts 5)
        (if (`/JukeboxMod/PDA_HeistSoundtrack.Stealth Only` _pdaheist)
          (`/Engine/EditorBlueprintResources/StandardMacros.IncrementInt` _stealthreselectattempts ; hack to prevent locking up the game
            (:`  `
              (goto _label_2)))
          (else
            _))
        (else
          (set `self.StealthReselectAttempts` 0)))
      (`/JukeboxMod/JukeboxFuncLibrary.PlaySong` _pdaheist)
      (`KismetSystemLibrary.Delay` (`KismetMathLibrary.RandomFloatInRange` 120.0 240.0))
      (if (not (`|EnumEquality` (`SBZGameStateMachineFunctionLibrary.GetGameStateMachineState`) "SM_Result"))
        (goto _label_2)))))

(fn `GetCurrentHeist`
  (returns (ValidHeist :type Boolean))
  (bind _returnvalue (`GameplayStatics.GetCurrentLevelName` true))
  (if (`PD3HeistDataAsset.bIsTutorialLevel` (`SBZHeistDeveloperSettings.GetHeistDataFromLevelShortName` _returnvalue))
    (`/PDML/Blueprints/Utilities/BPFL_ModLoader.PrintToModLoader` "In Tutorial")
    (return false)
    (else
      (set `/JukeboxMod/HeistSoundtrackPersistentObject.HeistIsRTC` (== (`SBZGameStateMachineSettings.LevelShortNameToIdx` _returnvalue) 3) (`self.As Heist Soundtrack Persistent Object`))
      (return true))))

(fn `HeistStateChangedEvent`
  (params (OldState :type "EPD3HeistState Enum" :default "Stealth") (NewState :type "EPD3HeistState Enum" :default "Stealth"))
  (`self.RTC_Fix`)
  (`self.RandomSongAssaultLogic` NewState))

(fn `RandomSongAssaultLogic`
  (params (Selection :type "EPD3HeistState Enum" :default "Stealth"))
  (bind _assaultactive (`self.AssaultActive`))
  (bind _stealthreselectattempts (`self.StealthReselectAttempts`))
  (bind _selection (`local.Selection`))
  (bind _pdaheist (`/JukeboxMod/HeistSoundtrackPersistentObject.PDAHeist` (`self.As Heist Soundtrack Persistent Object`)))
  (if (`/JukeboxMod/PDA_HeistSoundtrack.Stealth Only` (`/JukeboxMod/HeistSoundtrackPersistentObject.PDAHeist` (`self.As Heist Soundtrack Persistent Object`)))
    ;[1 1 1] i could change this to one branch node but i dont care
    (if (`KismetMathLibrary.BooleanNOR` (`|EnumEquality` _selection "Stealth") (`|EnumEquality` _selection "Search"))
      (`/JukeboxMod/JukeboxFuncLibrary.SelectRandomTrack` :!label _label)
      (if (<= _stealthreselectattempts 6)
        (if (`/JukeboxMod/PDA_HeistSoundtrack.Stealth Only` _pdaheist)
          (`/Engine/EditorBlueprintResources/StandardMacros.IncrementInt` _stealthreselectattempts ; hack to prevent locking up the game
            (:`  `
              (goto _label)))
          (else
            _))
        (else
          (set `self.StealthReselectAttempts` 0)))
      (`/JukeboxMod/JukeboxFuncLibrary.PlaySong` _pdaheist)
      (`/PDML/Blueprints/Utilities/BPFL_ModLoader.PrintToModLoader` (`KismetStringLibrary.Conv_BoolToString` (`self.AssaultActive`))))
    (elif (`/JukeboxMod/HeistSoundtrackPersistentObject.assaultRandomSong` (`self.As Heist Soundtrack Persistent Object`))
      (switch `EPD3HeistState` Selection
        (:`Assault`
          (if (not _assaultactive)
            (set `self.AssaultActive` true)))
        (:`Control`
          (if _assaultactive
            (set `self.AssaultActive` false)
            (goto _label)))))))

(fn `RTC_Fix`
  (bind _as_heist_soundtrack_persistent_object (`self.As Heist Soundtrack Persistent Object`))
  (bind _returnvalue (`PD3HeistGameState.GetCurrentHeistState` (`self.PD3HeistGameState`)))
  (if (and (not (`self.RTC_FixActive`)) (not (`/JukeboxMod/HeistSoundtrackPersistentObject.disableRTCFix` _as_heist_soundtrack_persistent_object)) (`/JukeboxMod/HeistSoundtrackPersistentObject.HeistIsRTC` _as_heist_soundtrack_persistent_object))
    (if (`/JukeboxMod/HeistSoundtrackPersistentObject.EnableRTCStealth` _as_heist_soundtrack_persistent_object)
      (`AkGameplayStatics.PostEventAtLocation` "/JukeboxMod/Music_Stop_Nightclub_Diagetic.Music_Stop_Nightclub_Diagetic" :!label _label)
      (elif (`KismetMathLibrary.BooleanNOR` (`|EnumEquality` _returnvalue "Stealth") (`|EnumEquality` _returnvalue "Search"))
        (set `self.RTC_FixActive` true)
        (goto _label)))))

(fn `SetupDebugStuff`
  (if (`/JukeboxMod/HeistSoundtrackPersistentObject.debug` (`self.As Heist Soundtrack Persistent Object`))
    (bind _returnvalue (`|CreateWidget` "/JukeboxMod/Widgets/JukeboxDebug.JukeboxDebug_C"))
    (`UserWidget.AddToViewport` _returnvalue 9999)))

(fn `SetupInHeistWidgets`
  (bind _returnvalue (`|CreateWidget` "/JukeboxMod/Widgets/JukeboxCurrentSong.JukeboxCurrentSong_C"))
  (`UserWidget.AddToViewport` _returnvalue 9999))

(fn `UserConstructionScript`)